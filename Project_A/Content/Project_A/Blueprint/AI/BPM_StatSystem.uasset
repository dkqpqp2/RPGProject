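; BPM_StatSystem is an AI stat Blueprint that tracks health and death state.
; On BeginPlay it fills CurrentHp to MaxHp through InitializeStat.
; IncreaseHp adds points and caps the result at MaxHp.
; DecreaseHp sets CurrentHp to damage minus current HP (operands reversed from a usual subtraction), then clamps negatives to zero, setting and returning IsDead in that case.
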(event EventBeginPlay
  (CallFunction|InitializeStat))

(event EventTick
  (params (DeltaSeconds :type Float%20%28single-precision%29)))

(fn IncreaseHp
  (params (HpPoint :type Float%20%28double-precision%29))
  (Variables|Default|SetCurrentHp (+ HpPoint (Variables|Default|GetCurrentHp)))
  (if (> (Variables|Default|GetCurrentHp) (Variables|Default|GetMaxHp))
    (Variables|Default|SetCurrentHp (Variables|Default|GetMaxHp))))

(fn DecreaseHp
  (params (DamagePoint :type Float%20%28double-precision%29))
  (Variables|Default|SetCurrentHp (- DamagePoint (Variables|Default|GetCurrentHp)))
  (if (< (Variables|Default|GetCurrentHp) 0.0)
    (Variables|Default|SetCurrentHp 0.0)
    (bind _output_get (Variables|Default|SetIsDead true))
    (return _output_get)))

(fn InitializeStat
  (Variables|Default|SetCurrentHp (Variables|Default|GetMaxHp)))